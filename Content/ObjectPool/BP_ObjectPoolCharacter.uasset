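; BP_ObjectPoolCharacter is a character Blueprint that fires pre-spawned bullets from an object pool on Space Bar press.
; It takes the bullet at BulletIndex from BPBulletPool, launches it along its forward vector at its ProjectileMovement initial speed, then detaches it in world space.
; BulletIndex advances after each valid shot and wraps to zero at the pool's length, cycling through the pool round-robin.
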(event Input|KeyboardEvents|SpaceBar
  (params (Key :type Key%20Structure :default "None"))
  (bind _bp_bulletpool (Variables|Default|GetBP_BulletPool))
  (bind _bulletpool (Variables|/Game/ObjectPool/BP_BulletPool.BP_BulletPool_C|GetBulletPool _bp_bulletpool))
  (bind _returnvalue (Utilities|Array|Length _bulletpool))
  (:Pressed
    (if (> _returnvalue 0)
      (Variables|Default|SetMaxPool _returnvalue)
      (Utilities|IsValid (Utilities|Array|Get(acopy) _bulletpool (Variables|Default|GetBulletIndex))
        (:Is%20Valid
          (Default|FireBullet (Utilities|Array|Get(acopy) _bulletpool (Variables|Default|GetBulletIndex)) (* (Transformation|GetActorForwardVector (Utilities|Array|Get(acopy) _bulletpool (Variables|Default|GetBulletIndex))) (Variables|/Script/Engine.ProjectileMovementComponent|GetInitialSpeed (Variables|/Game/ObjectPool/BP_Bullet.BP_Bullet_C|GetProjectileMovement (Utilities|Array|Get(acopy) _bulletpool (Variables|Default|GetBulletIndex))))))
          (Transformation|DetachFromActor (Utilities|Array|Get(acopy) _bulletpool (Variables|Default|GetBulletIndex)) "KeepWorld" "KeepWorld" "KeepWorld")
          (bind _result (Math|Integer|IncrementInt (Variables|Default|GetBulletIndex))
            (:%20%20
              (bind _output_get (Variables|Default|SetBulletIndex _result))
              (if (== _output_get (Variables|Default|GetMaxPool))
                (Variables|Default|SetBulletIndex 0)))))))))

(fn ConstructionScript)