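; Bullet pool that pre-spawns BP_Bullet actors at its owner's location on BeginPlay for reuse.
; Each bullet has mesh collision disabled, is attached to the owner, stored in the BulletPool array and bound to its OnBulletDestroyed event.
; That event calls ReturnToThePool, which moves the bullet back to the owner and reattaches it.
; Logic for taking bullets from the pool is not in this graph.
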(event Custom|ReturnToThePool
  (params (Bullet :type BP%20Bullet%20Object%20Reference))
  (Transformation|SetActorLocation Bullet (Transformation|GetActorLocation (Components|GetOwner)) false false)
  (Transformation|AttachActorToActor Bullet (Components|GetOwner) "None" "KeepWorld" "KeepWorld" "KeepWorld" true))

(event EventBeginPlay
  (for _index (range 0 (Variables|Default|GetAmountOfBullets))
    (bind _returnvalue (Game|SpawnActorfromClass "/Game/ObjectPool/BP_Bullet.BP_Bullet_C" (Math|Transform|MakeTransform (Transformation|GetActorLocation (Components|GetOwner)) "0, 0, 0" "1.000000,1.000000,1.000000") "Undefined" "MultiplyWithRoot" 0 0))
    (Collision|SetCollisionEnabled (Variables|/Game/ObjectPool/BP_Bullet.BP_Bullet_C|GetStaticMesh _returnvalue) "NoCollision")
    (Transformation|AttachActorToActor _returnvalue (Components|GetOwner) "None" "KeepWorld" "KeepWorld" "KeepWorld" true)
    (EventDispatchers|AssignOnBulletDestroyed _returnvalue (delegate Custom|ReturnToThePool))
    (Utilities|Array|Add (Variables|Default|GetBulletPool) _returnvalue)))