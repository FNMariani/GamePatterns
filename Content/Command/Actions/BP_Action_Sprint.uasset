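; Sprint action in a start/stop action system that temporarily raises the acting character's movement speed.
; On start, it runs the parent logic, then adds BonusSpeed to the MaxWalkSpeed of the actor's CharacterMovementComponent.
; On stop, it runs the parent logic, then subtracts BonusSpeed, so the change is relative to the current speed rather than a cached original.
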(event EventStartAction
  (params (Actor :type Actor%20Object%20Reference))
  (bind _returnvalue (Actor|GetComponentbyClass Actor "/Script/Engine.CharacterMovementComponent"))
  (|CallParentFunction Actor)
  (Variables|/Script/Engine.CharacterMovementComponent|SetMaxWalkSpeed _returnvalue (+ (Variables|/Script/Engine.CharacterMovementComponent|GetMaxWalkSpeed _returnvalue) (Variables|Default|GetBonusSpeed))))

(event EventStopAction
  (params (Actor :type Actor%20Object%20Reference))
  (bind _returnvalue (Actor|GetComponentbyClass Actor "/Script/Engine.CharacterMovementComponent"))
  (|CallParentFunction Actor)
  (Variables|/Script/Engine.CharacterMovementComponent|SetMaxWalkSpeed _returnvalue (- (Variables|/Script/Engine.CharacterMovementComponent|GetMaxWalkSpeed _returnvalue) (Variables|Default|GetBonusSpeed))))